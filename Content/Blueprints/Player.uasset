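; Player character for a cursor-aimed game, handling movement, sprint stamina, health with level load on death, and stamina/health widgets.
; Each tick it faces the cursor and builds line-of-sight vision from a fan of line traces, drawn as triangles into a render target, with position published to a material parameter collection.
; Holding left mouse charges a capped damage value that is never applied; interact and M-key self-damage are test hooks.
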(event Custom|Charge%20Attack
  ;[1 1 1] axe charge attack
  (if (stale Input|MouseEvents|LeftMouseButton _output_get)
    (Variables|Combat|SetDamage (Math|Float|Clamp(Float) (+ (Variables|Combat|GetDamage) 1.0) 0.0 2e+01))
    (Utilities|FlowControl|Delay 0.3)
    (CallFunction|ChargeAttack)))

(event Custom|IncreaseStamina
  ;[0 0 0] Stamina
  (Variables|PlayerStats|SetStamina (+ (Variables|PlayerStats|GetStamina) 2.0))
  (if (>= (Variables|PlayerStats|GetStamina) 1e+02)
    (Variables|Movement|SetcanIncreaseStamina false :!label _label)
    (elif (Variables|Movement|GetisRunning?)
      (goto _label)
      (else
        (Variables|Movement|SetcanIncreaseStamina true)))))

(event Custom|UseStamina
  ;[0 0 0] Stamina
  (Variables|PlayerStats|SetStamina (- (Variables|PlayerStats|GetStamina) 5.0))
  (if (<= (Variables|PlayerStats|GetStamina) 0.0)
    (Variables|Movement|SetisRunning? false)
    (Variables|/Script/Engine.CharacterMovementComponent|SetMaxWalkSpeed (Variables|Character|GetCharacterMovement) (Variables|Movement|GetwalkSpeed))
    (else
      (Development|PrintString (Utilities|String|ToString(Float) (Variables|PlayerStats|GetStamina))))))

(event Input|EnhancedActionEvents|EnhancedInputActionIA_Movement
  (params (ActionValue :type Vector%202D%20Structure) (ElapsedSeconds :type Float%20%28double-precision%29) (TriggeredSeconds :type Float%20%28double-precision%29) (InputAction :type Input%20Action%20Object%20Reference :default "/Game/Input/IA_Movement.IA_Movement"))
  ;[0 0 0] Move left/right
  (Pawn|Input|AddMovementInput (Math|Vector|GetRightVector (Math|Rotator|MakeRotator 0.0 0.0 (.yaw (Pawn|GetControlRotation :!class /Script/Engine.Pawn)))) (.x ActionValue) false)
  ;[0 0 0] Move Forward/ back
  (Pawn|Input|AddMovementInput (Math|Vector|GetForwardVector (Math|Rotator|MakeRotator 0.0 0.0 (.yaw (Pawn|GetControlRotation :!class /Script/Engine.Pawn)))) (.y ActionValue) false))

(event Input|EnhancedActionEvents|EnhancedInputActionIA_interact
  (params (ActionValue :type Boolean) (ElapsedSeconds :type Float%20%28double-precision%29) (TriggeredSeconds :type Float%20%28double-precision%29) (InputAction :type Input%20Action%20Object%20Reference :default "/Game/Input/IA_interact.IA_interact"))
  (bind _current_test_item (Variables|Default|GetCurrent%20Test%20Item))
  ;[0 0 0] Interaction test
  (Utilities|IsValid _current_test_item
    (:Is%20Valid
      (Actor|DestroyActor _current_test_item))
    (:Is%20Not%20Valid
      (Development|PrintString "No interaction"))))

(event EventBeginPlay
  (Utilities|FlowControl|Sequence
    (:then_0
      ;[0 0 0] Movement Controller
      (bind _asplayer_controller_1 (Utilities|Casting|CastToPlayerController1 (Pawn|GetController)))
      (Utilities|IsValid (PlayerController|LocalPlayerSubsystems|GetEnhancedInputLocalPlayerSubsystem _asplayer_controller_1)
        (:Is%20Valid
          (Input|AddMappingContext (PlayerController|LocalPlayerSubsystems|GetEnhancedInputLocalPlayerSubsystem _asplayer_controller_1) "/Game/Input/IMC_Default.IMC_Default" 0 "(bIgnoreAllPressedKeysUntilRelease=True,bForceImmediately=False,bNotifyUserSettings=False)")
          (Variables|/Script/Engine.PlayerController|SetbShowMouseCursor (Game|GetPlayerController 0) true))))
    (:then_1
      ;[0 0 0] Stamina UI
      (bind _returnvalue (UserInterface|CreateWidget "/Game/UI/WP_Stamina.WP_Stamina_C" (Game|GetPlayerController 0)))
      (UserInterface|Viewport|AddtoViewport _returnvalue 0))
    (:then_2
      ;[0 0 0] Health UI
      (bind _returnvalue_2 (UserInterface|CreateWidget "/Game/UI/WP_Health.WP_Health_C" (Game|GetPlayerController 0)))
      (UserInterface|Viewport|AddtoViewport _returnvalue_2 0))
    (:then_3
      (Variables|/Script/Engine.CharacterMovementComponent|SetMaxWalkSpeed (Variables|Character|GetCharacterMovement) (Variables|Movement|GetwalkSpeed)))))

(event EventTick
  (params (DeltaSeconds :type Float%20%28single-precision%29))
  (Utilities|FlowControl|Sequence
    (:then_0
      ;[0 0 0] Rotation
      (Transformation|SetActorRotation (Math|Rotator|MakeRotator 0.0 0.0 (.yaw (Math|Rotator|FindLookatRotation (Transformation|GetActorLocation) (.location (.HitResult (Game|Player|GetHitResultUnderCursorbyChannel (Game|GetPlayerController 0) "TraceTypeQuery1" true))))))))
    (:then_1
      (CallFunction|LosVisionSystem))
    (:then_2
      (Variables|Movement|SetisMoving? (> (Math|Vector|VectorLength (Transformation|GetVelocity)) 0.0)))))

(event Game|Damage|EventAnyDamage
  (params (Damage :type Float%20%28single-precision%29) (DamageType :type Damage%20Type%20Object%20Reference) (InstigatedBy :type Controller%20Object%20Reference) (DamageCauser :type Actor%20Object%20Reference))
  ;[0 0 0] Health System
  (Variables|PlayerStats|Sethealth (- (Variables|PlayerStats|Gethealth) Damage))
  (if (<= (Variables|PlayerStats|Gethealth) 0.0)
    (Development|PrintString "Dead")
    (Game|OpenLevel(byObjectReference) "/Game/NightStalkermain.NightStalkermain")
    (else
      (Development|PrintString (Utilities|String|ToString(Float) (Variables|PlayerStats|Gethealth))))))

(event Input|MouseEvents|LeftMouseButton
  (params (Key :type Key%20Structure :default "None"))
  (:Pressed
    (Utilities|FlowControl|Sequence
      (:then_0
        ;[1 1 1] axe charge attack
        (if true
          (bind _output_get (Variables|Combat|SetCharging true))
          (if _output_get
            (Variables|Combat|SetDamage (Math|Float|Clamp(Float) (+ (Variables|Combat|GetDamage) 1.0) 0.0 2e+01))
            (Utilities|FlowControl|Delay 0.3)
            (CallFunction|ChargeAttack))))))
  (:Released
    (Variables|Combat|SetCharging false)))

(event Input|KeyboardEvents|LeftShift
  (params (Key :type Key%20Structure :default "None"))
  (bind _charactermovement (Variables|Character|GetCharacterMovement))
  ;[0 0 0] Stamina
  (:Pressed
    (Variables|Movement|SetisRunning? true)
    (Variables|/Script/Engine.CharacterMovementComponent|SetMaxWalkSpeed _charactermovement (Variables|Movement|GetrunSpeed) :!label _label)
    (if (Variables|Movement|GetisMoving?)
      (Utilities|FlowControl|RetriggerableDelay 0.2)
      (CallFunction|UseStamina)
      (if (Variables|Movement|GetisRunning?)
        (goto _label))))
  (:Released
    (Variables|Movement|SetisRunning? false)
    (Variables|/Script/Engine.CharacterMovementComponent|SetMaxWalkSpeed _charactermovement (Variables|Movement|GetwalkSpeed) :!label _label_2)
    (Utilities|FlowControl|RetriggerableDelay 0.2)
    (CallFunction|IncreaseStamina)
    (if (Variables|Movement|GetcanIncreaseStamina)
      (goto _label_2))))

(event Input|KeyboardEvents|M
  (params (Key :type Key%20Structure :default "None"))
  ;[0 0 0] Test Damage (press M)
  (:Pressed
    (Game|Damage|ApplyDamage self 1e+01 0 0)))

(fn ConstructionScript)

(fn LosVisionSystem
  (bind _losrendertarget (Variables|Vision|GetLosRenderTarget))
  (Utilities|FlowControl|Sequence
    (:then_0
      (Rendering|Material|SetVectorParameterValue "/Game/PlayerVision/PlayerPos.PlayerPos" "PlayerPosition" (Math|Conversions|ToLinearColor(Vector) (Transformation|GetActorLocation)) :!class /Script/Engine.KismetMaterialLibrary))
    (:then_1
      (CallFunction|CreateCone))
    (:then_2
      (CallFunction|PrepareTrianglesforCanvas))
    (:then_3
      (Rendering|ClearRenderTarget2D _losrendertarget)
      (bind (_canvas _size _context) (Rendering|BeginDrawCanvastoRenderTarget _losrendertarget))
      (Class|Canvas|DrawTriangle _canvas 0 (Variables|Vision|GetCanvasTriangles))
      (Rendering|EndDrawCanvastoRenderTarget _context))))

(fn CreateCone
  (bind _returnvalue (Transformation|GetActorLocation))
  (bind _traceresults (Variables|Vision|GetTraceResults))
  (Utilities|Array|Clear (Variables|Vision|GetTraceResults))
  (for _index (range 0 (Variables|Vision|GetNumTraces))
    (bind (_outhit _returnvalue_2) (Collision|LineTraceByChannel _returnvalue (+ (* (Math|Vector|RotateVector (Math|Vector|RotateVector (Transformation|GetActorForwardVector) (Math|Rotator|MakeRotator 0.0 0.0 (/ (* (Variables|Vision|GetNumTraces) (Variables|Vision|GetDegreesPerTrace)) -2.0))) (Math|Rotator|MakeRotator 0.0 0.0 (* _index (Variables|Vision|GetDegreesPerTrace)))) 1e+03) _returnvalue) "TraceTypeQuery1" false 0 "None"))
    (if _returnvalue_2
      (Utilities|Array|Add _traceresults (+ (* (Math|Vector|RotateVector (Math|Vector|RotateVector (Transformation|GetActorForwardVector) (Math|Rotator|MakeRotator 0.0 0.0 (/ (* (Variables|Vision|GetNumTraces) (Variables|Vision|GetDegreesPerTrace)) -2.0))) (Math|Rotator|MakeRotator 0.0 0.0 (* _index (Variables|Vision|GetDegreesPerTrace)))) 2.0) (.location _outhit)))
      (else
        (Utilities|Array|Add _traceresults (+ (* (Math|Vector|RotateVector (Math|Vector|RotateVector (Transformation|GetActorForwardVector) (Math|Rotator|MakeRotator 0.0 0.0 (/ (* (Variables|Vision|GetNumTraces) (Variables|Vision|GetDegreesPerTrace)) -2.0))) (Math|Rotator|MakeRotator 0.0 0.0 (* _index (Variables|Vision|GetDegreesPerTrace)))) 2.0) (+ (* (Math|Vector|RotateVector (Math|Vector|RotateVector (Transformation|GetActorForwardVector) (Math|Rotator|MakeRotator 0.0 0.0 (/ (* (Variables|Vision|GetNumTraces) (Variables|Vision|GetDegreesPerTrace)) -2.0))) (Math|Rotator|MakeRotator 0.0 0.0 (* _index (Variables|Vision|GetDegreesPerTrace)))) 1e+03) _returnvalue)))))))

(fn PrepareTrianglesforCanvas
  (bind _returnvalue (Transformation|GetActorLocation))
  (bind _returnvalue_2 (Math|Vector|MakeVector 9e+02 9e+02 0.0))
  (bind _traceresults (Variables|Vision|GetTraceResults))
  (Utilities|Array|Clear (Variables|Vision|GetCanvasTriangles))
  (for _index (range 0 (- (Utilities|Array|Length (Variables|Vision|GetTraceResults)) 2))
    (Utilities|Array|Add (Variables|Vision|GetCanvasTriangles) (Utilities|Struct|MakeCanvasUVTri (Math|Conversions|ToVector2D(Vector) _returnvalue_2) "(X=0.000000,Y=0.000000)" "(R=1.000000,G=1.000000,B=1.000000,A=0.000000)" (Math|Conversions|ToVector2D(Vector) (+ (- (Utilities|Array|Get(acopy) _traceresults _index) _returnvalue) _returnvalue_2)) "(X=0.000000,Y=0.000000)" "(R=1.000000,G=1.000000,B=1.000000,A=0.000000)" (Math|Conversions|ToVector2D(Vector) (+ (- (Utilities|Array|Get(acopy) _traceresults (+ _index 1)) _returnvalue) _returnvalue_2)) "(X=0.000000,Y=0.000000)" "(R=1.000000,G=1.000000,B=1.000000,A=0.000000)"))))

(fn UseStamina)