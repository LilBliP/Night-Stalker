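; TestItem is a test actor that registers itself with the Player when the player overlaps it.
; On begin overlap it sets the player's CurrentTestItem to itself, and on end overlap clears that reference only if it still points to this item.
; A DestroyItem function destroys the actor.
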(event Collision|EventActorBeginOverlap
  (params (OtherActor :type Actor%20Object%20Reference))
  (bind _asplayer (Utilities|Casting|CastToPlayer OtherActor))
  (Variables|/Game/Playercharacter/Player.Player_C|SetCurrent%20Test%20Item _asplayer self))

(event Collision|EventActorEndOverlap
  (params (OtherActor :type Actor%20Object%20Reference))
  (bind _asplayer (Utilities|Casting|CastToPlayer OtherActor))
  (if (== (Variables|/Game/Playercharacter/Player.Player_C|GetCurrent%20Test%20Item _asplayer) self)
    (Variables|/Game/Playercharacter/Player.Player_C|SetCurrent%20Test%20Item _asplayer 0)))

(fn ConstructionScript)

(fn DestroyItem
  (Actor|DestroyActor))